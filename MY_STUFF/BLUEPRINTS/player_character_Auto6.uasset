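; Player character Blueprint with flipbook-sprite animation states, yaw-relative movement and a sprint input.
; Movement axis events add input and call updateAnimation, which derives movement from velocity and runs AnimationStateMachine to pick Idle, Walking or Running.
; The chosen flipbook is returned but never applied, as SetFlipbook is unwired; the aimed selection is unused.
; Sprint switches walk speed, but releasing it never clears IsSprinting.
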(event `updateAnimation`
  (bind _returnvalue (`KismetMathLibrary.VSize` (`self.GetVelocity`)))
  (set `self.currentSpeed` _returnvalue)
  (set `self.isMoving` (> _returnvalue 0.0))
  (`self.animationStateMachine`))

(event `InputAction|Sprint`
  (params (Key :type "Key Structure"))
  (bind _charactermovement (`self.CharacterMovement`))
  (:`Pressed`
    (set `CharacterMovementComponent.MaxWalkSpeed` (`self.RunSpeed`) _charactermovement)
    (set `self.isSprinting` true))
  (:`Released`
    (set `CharacterMovementComponent.MaxWalkSpeed` (`self.WalkSpeed`) _charactermovement)))

(event `InputAxis|MoveForward`
  (params (AxisValue :type "Float (single-precision)"))
  (`self.AddMovementInput` (`KismetMathLibrary.GetForwardVector` (`KismetMathLibrary.MakeRotator` 0.0 0.0 (.yaw (`self.GetControlRotation`)))) AxisValue)
  (`self.updateAnimation` :!label _label))

(event `InputAxis|MoveRight`
  (params (AxisValue :type "Float (single-precision)"))
  (`self.AddMovementInput` (`KismetMathLibrary.GetRightVector` (`KismetMathLibrary.MakeRotator` 0.0 0.0 (.yaw (`self.GetControlRotation`)))) AxisValue)
  (goto _label))

(fn `animationStateMachine`
  (returns (flipBook :type "PaperFlipbook Object Reference") (ReturnValue :type "PaperFlipbook Object Reference"))
  (if (`self.isMoving`)
    (if (`self.isSprinting`)
      (set `self.AS_normal` "NewEnumerator2")
      (set `self.AS_Aimed` "NewEnumerator2")
      (else
        (set `self.AS_normal` "NewEnumerator1")
        (set `self.AS_Aimed` "NewEnumerator1")))
    (else
      (set `self.AS_normal` "NewEnumerator0")
      (set `self.AS_Aimed` "NewEnumerator0")))
  (return (select `/Game/MY_STUFF/BLUEPRINTS/AS_normal` (`self.AS_normal`) :`NewEnumerator0` (`self.idle`) :`NewEnumerator1` (`self.walking`) :`NewEnumerator2` (`self.running`)) null))

(fn `UserConstructionScript`)