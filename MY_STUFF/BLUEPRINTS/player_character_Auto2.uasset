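; Player character Blueprint that handles walking, strafing and sprinting input.
; Move axes add movement input along forward and right vectors built from control rotation yaw only, keeping movement independent of camera pitch.
; The Sprint action sets the movement component's max walk speed to RunSpeed while held and restores WalkSpeed on release.
; BeginPlay, overlap, Tick and construction script are empty.
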(event `InputAction|Sprint`
  (params (Key :type "Key Structure"))
  (bind _charactermovement (`self.CharacterMovement`))
  (:`Pressed`
    (set `CharacterMovementComponent.MaxWalkSpeed` (`self.RunSpeed`) _charactermovement))
  (:`Released`
    (set `CharacterMovementComponent.MaxWalkSpeed` (`self.WalkSpeed`) _charactermovement)))

(event `InputAxis|MoveForward`
  (params (AxisValue :type "Float (single-precision)"))
  (`self.AddMovementInput` (`KismetMathLibrary.GetForwardVector` (`KismetMathLibrary.MakeRotator` 0.0 0.0 (.yaw (`self.GetControlRotation`)))) AxisValue))

(event `InputAxis|MoveRight`
  (params (AxisValue :type "Float (single-precision)"))
  (`self.AddMovementInput` (`KismetMathLibrary.GetRightVector` (`KismetMathLibrary.MakeRotator` 0.0 0.0 (.yaw (`self.GetControlRotation`)))) AxisValue))

(fn `UserConstructionScript`)